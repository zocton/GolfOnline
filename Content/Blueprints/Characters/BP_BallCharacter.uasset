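; Ball character Blueprint that shows a Niagara effect while the Boost input is held; no boost movement is applied here.
; Pressing adds a component, attaches it to Ball, advances its simulation and prints debug text, while releasing destroys it.
; Tick draws a debug circle at the root, and construction gives the Absolute component world-space rotation.
; An alternative NS_Boost spawn behind Absolute is left unconnected.
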(event EventTick
  (params (DeltaSeconds :type Float%20%28single-precision%29))
  (Rendering|Debug|DrawDebugCircle (Transformation|GetWorldLocation (Variables|Transformation|GetRootComponent)) 2e+01 12 "(R=0.000000,G=1.000000,B=0.000000,A=1.000000)" 0.0 0.0 "0.000000,1.000000,0.000000" "0.000000,0.000000,1.000000"))

(event Input|ActionEvents|InputActionBoost
  (params (Key :type Key%20Structure :default "None"))
  (:Pressed
    (bind _returnvalue (AddComponent|AddNiagaraComponent true))
    (Transformation|AttachComponentToComponent _returnvalue (Variables|Default|GetBall) "None" "KeepRelative" "KeepRelative" "KeepRelative" true)
    (Class|NiagaraComponent|AdvanceSimulationbyTime _returnvalue 1.0 (stale EventTick DeltaSeconds))
    (Development|PrintString "Hello"))
  (:Released
    (Components|DestroyComponent _returnvalue)))

(fn ConstructionScript
  (Variables|/Script/Engine.SceneComponent|SetbAbsoluteRotation (Variables|Default|GetAbsolute) true))